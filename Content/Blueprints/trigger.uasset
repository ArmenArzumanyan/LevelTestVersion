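; Trigger Blueprint that activates and deactivates a message on a linked actor when something enters or leaves its box volume.
; Box begin overlap calls AtivateMessage on the ActorTolnteract reference and prints success or failure from its return value.
; End overlap calls DeactivateMessage, but its branch condition is fixed true, so it always prints the deactivate text.
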(event `self.Box.OnComponentBeginOverlap`
  (params (OverlappedComponent :type "PrimitiveComponent Object Reference") (OtherActor :type "Actor Object Reference") (OtherComp :type "PrimitiveComponent Object Reference") (OtherBodyIndex :type Integer) (bFromSweep :type Boolean) (SweepResult :type "HitResult Structure (by ref)"))
  (bind _succses (message `/Game/Blueprints/bpi_avtivation.Ativate` (`self.actorTolnteract`)))
  (if _succses
    (`KismetSystemLibrary.PrintString` "activaed")
    (else
      (`KismetSystemLibrary.PrintString` "Active Fail."))))

(event `self.Box.OnComponentEndOverlap`
  (params (OverlappedComponent :type "PrimitiveComponent Object Reference") (OtherActor :type "Actor Object Reference") (OtherComp :type "PrimitiveComponent Object Reference") (OtherBodyIndex :type Integer))
  (message `/Game/Blueprints/bpi_avtivation.Deactivate` (`self.actorTolnteract`))
  (if true
    (`KismetSystemLibrary.PrintString` "deactivate")
    (else
      (`KismetSystemLibrary.PrintString` "Deactivate  Fail/"))))

(fn `UserConstructionScript`)