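; Fan actor that spins while its enable flag is set.
; Tick adds a fixed local pitch rotation each frame without delta-time scaling, so spin speed depends on frame rate.
; The Ativate and Deactivate functions set or clear the flag, print a debug message and return true.
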(event `self.ReceiveTick`
  (params (DeltaSeconds :type "Float (single-precision)"))
  (if (`self.fanEnable`)
    (`self.K2_AddActorLocalRotation` (`KismetMathLibrary.MakeRotator` 0.0 15.0))))

(fn `Ativate`
  (returns (Succses :type Boolean))
  (`KismetSystemLibrary.PrintString` "fan  eneable is true")
  (set `self.fanEnable` true)
  (return true))

(fn `Deactivate`
  (returns (Sucsses :type Boolean))
  (`KismetSystemLibrary.PrintString` "fan  eneable is false" true true (struct :`G` 0.66 :`B` 1.0 :`A` 1.0) 5.0)
  (set `self.fanEnable` false)
  (return true))

(fn `UserConstructionScript`)